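; Game mode Blueprint for Toon Tanks that puts the match start and end screens on screen.
; GameStart creates the WBP_GameStart widget, passes it StartDelay and adds it to the viewport.
; GameOver creates WBP_GameEnd, passes it the PlayerWon result and adds it to the viewport.
; Both widgets are kept in variables, and the graph holds no other game rules.
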(event EventGameStart
  (bind _returnvalue (UserInterface|CreateWidget "/Game/Blueprints/Widgets/WBP_GameStart.WBP_GameStart_C"))
  (Variables|Default|SetGameStartWidget _returnvalue)
  (Default|SetStartDelay (Variables|Default|GetGameStartWidget) (Variables|Default|GetStartDelay))
  (UserInterface|Viewport|AddtoViewport (Variables|Default|GetGameStartWidget) 0))

(event EventGameOver
  (params (PlayerWon :type Boolean))
  (bind _returnvalue (UserInterface|CreateWidget "/Game/Blueprints/Widgets/WBP_GameEnd.WBP_GameEnd_C"))
  (Variables|Default|SetEndGameWidget _returnvalue)
  (Default|SetPlayerWon (Variables|Default|GetEndGameWidget) PlayerWon)
  (UserInterface|Viewport|AddtoViewport (Variables|Default|GetEndGameWidget) 0))

(fn ConstructionScript)